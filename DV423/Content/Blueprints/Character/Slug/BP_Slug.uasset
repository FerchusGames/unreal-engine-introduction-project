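; BP_Slug is a slug character actor that continuously turns to face the player character.
; Each tick, RotateTowardsMainCharacter checks that player 0's character is a BP_CharacterBase, then applies the rotation from GetLookAtRotation.
; That helper keeps only the yaw of the look-at rotation and eases toward it with RInterpTo, so the slug stays upright and turns smoothly.
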(event `self.ReceiveTick`
  (params (DeltaSeconds :type "Float (single-precision)"))
  (`self.Rotate Towards Main Character`))

(fn `Get Look At Rotation`
  (params (Target :type "Actor Object Reference"))
  (returns (`Look Rotation` :type "Rotator Structure"))
  (bind (_returnvalue_roll _returnvalue_pitch _returnvalue_yaw) (`KismetMathLibrary.BreakRotator` (`KismetMathLibrary.FindLookAtRotation` (`self.K2_GetActorLocation`) (`self.K2_GetActorLocation` Target))))
  (return (`KismetMathLibrary.RInterpTo` (`self.K2_GetActorRotation`) (`KismetMathLibrary.MakeRotator` 0.0 0.0 _returnvalue_yaw) (`GameplayStatics.GetWorldDeltaSeconds`) 3.0)))

(fn `Rotate Towards Main Character`
  (bind _returnvalue (`GameplayStatics.GetPlayerCharacter` 0))
  (cast `/Game/Blueprints/Character/BP_CharacterBase` _returnvalue)
  (bind _look_rotation (`self.Get Look At Rotation` _returnvalue))
  (`self.K2_SetActorRotation` _look_rotation))

(fn `UserConstructionScript`)