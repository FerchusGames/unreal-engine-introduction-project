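; Player controller that turns movement, jump and mouse look input into actions on the controlled pawn.
; Move axes add movement input along the camera manager's forward and right vectors, using the full camera rotation rather than yaw alone.
; Mouse axes feed yaw and pitch input directly, and Jump acts only when the pawn casts to Character.
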(event `InputAxis|Move Forward / Backward`
  (params (AxisValue :type "Float (single-precision)"))
  ;[1 1 1] Player Movement
  (`self.Move Forward / Backward` AxisValue))

(event `InputAxis|Move Right / Left`
  (params (AxisValue :type "Float (single-precision)"))
  ;[1 1 1] Player Movement
  (`self.Move Right / Left` AxisValue))

(event `InputAction|Jump`
  (params (Key :type "Key Structure"))
  ;[1 1 1] Player Movement
  (:`Pressed`
    (`self.Jump`)))

(event `InputAxis|Turn Right / Left Mouse`
  (params (AxisValue :type "Float (single-precision)"))
  ;[1 1 1] Camera Movement
  (`self.AddYawInput` AxisValue))

(event `InputAxis|Look Up / Down Mouse`
  (params (AxisValue :type "Float (single-precision)"))
  ;[1 1 1] Camera Movement
  (`self.AddPitchInput` AxisValue))

(fn `Jump`
  (bind _ascharacter (cast `Character` (`self.K2_GetPawn`)))
  (`Character.Jump` _ascharacter))

(fn `Move Forward / Backward`
  (params (ScaleValue :type "Float (single-precision)"))
  (`Pawn.AddMovementInput` (`self.K2_GetPawn`) (`KismetMathLibrary.GetForwardVector` (`PlayerCameraManager.GetCameraRotation` (`self.PlayerCameraManager`))) ScaleValue false))

(fn `Move Right / Left`
  (params (ScaleValue :type "Float (single-precision)"))
  (`Pawn.AddMovementInput` (`self.K2_GetPawn`) (`KismetMathLibrary.GetRightVector` (`PlayerCameraManager.GetCameraRotation` (`self.PlayerCameraManager`))) ScaleValue false))

(fn `UserConstructionScript`)