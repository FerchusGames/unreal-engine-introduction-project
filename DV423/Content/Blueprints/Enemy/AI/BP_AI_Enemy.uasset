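; AI controller for enemies that runs the BT_Enemies behavior tree when it possesses a BP_Enemy.
; AI perception updates on BP_CharacterBase actors write the sensed state to the CanSeePlayer blackboard key.
; A FindThePlayer move-to event remains, but its looping timer is disconnected and never runs.
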(event `self.ReceiveBeginPlay`)

(event `FindThePlayer`
  (`|AIMoveTo` (`self.K2_GetPawn`) (0.0 0.0 0.0) (`GameplayStatics.GetPlayerController` 0) 100.0))

(event `self.ReceivePossess`
  (params (PossessedPawn :type "Pawn Object Reference"))
  (cast `/Game/Blueprints/Enemy/BP_Enemy` PossessedPawn)
  (`self.RunBehaviorTree` "/Game/Blueprints/Enemy/AI/BT_Enemies.BT_Enemies"))

(event `self.AIPerception.OnTargetPerceptionUpdated`
  (params (Actor :type "Actor Object Reference") (Stimulus :type "AIStimulus Structure"))
  (cast `/Game/Blueprints/Character/BP_CharacterBase` Actor)
  (`BlackboardComponent.SetValueAsBool` (`self.Blackboard`) "CanSeePlayer" (`.bSuccessfullySensed` (break `AIStimulus` Stimulus))))

(fn `UserConstructionScript`)